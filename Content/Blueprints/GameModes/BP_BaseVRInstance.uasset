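; VR game instance that enables the HMD on init and handles hosting and joining of multiplayer sessions.
; Hosting creates a four-connection session, with LAN use set by a variable, then opens the Destructible level as a listen server.
; Joining searches for sessions and connects to the first result, without any selection step.
; Failures and empty searches are only reported through printed debug strings.
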(event `self.ReceiveInit`
  (`HeadMountedDisplayFunctionLibrary.EnableHMD` true))

(event `HostGameEvent`
  (`CreateSessionCallbackProxy.CreateSession` (`GameplayStatics.GetPlayerController` 0) 4 (`self.EnableLAN`)
    (:`OnSuccess`
      (`GameplayStatics.OpenLevel` "Destructible" true "listen"))
    (:`OnFailure`
      (`KismetSystemLibrary.PrintString` "Failed to create session"))))

(event `JoinSession`
  (bind _results (`FindSessionsCallbackProxy.FindSessions` (`GameplayStatics.GetPlayerController` 0) 10 (`self.EnableLAN`))
    (:`OnSuccess`
      (if (== (`KismetArrayLibrary.Array_Length` _results) 0)
        (`KismetSystemLibrary.PrintString` "No sessions found")
        (else
          (bind _asplayer_controller (cast `PlayerController` (`Pawn.GetController` (`GameplayStatics.GetPlayerPawn` 0))))
          (`JoinSessionCallbackProxy.JoinSession` _asplayer_controller (`|GetArrayItem` _results)
            (:`OnFailure`
              (`KismetSystemLibrary.PrintString` "Failed to join session"))))))
    (:`OnFailure`
      (`KismetSystemLibrary.PrintString` "Rip"))))