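; BaseVRMode is a game mode that spawns VR motion controller pawns for players as they log in.
; On PostLogin, the authority caches all PlayerStart actors and calls RespawnPlayer, which destroys any existing pawn, then spawns and possesses a new MotionControllerPawn.
; The player whose ID matches the first PlayerArray entry spawns at the first found start; every other player uses the second.
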(event `RespawnPlayer`
  (params (PlayerController :type "PlayerController Object Reference"))
  (bind _returnvalue (`Controller.K2_GetPawn` PlayerController))
  (`/Engine/EditorBlueprintResources/StandardMacros.IsValid` _returnvalue
    (:`Is Valid`
      (`self.K2_DestroyActor` _returnvalue))
    (:`Is Not Valid`
      _))
  (if (== (`PlayerState.PlayerId` (`Controller.PlayerState` PlayerController)) (`PlayerState.PlayerId` (`|GetArrayItem` (`GameStateBase.PlayerArray` (`GameplayStatics.GetGameState`)))))
    (bind _returnvalue_2 (`|SpawnActorFromClass` "/Game/VirtualRealityBP/Blueprints/MotionControllerPawn.MotionControllerPawn_C" (`self.GetTransform` (`|GetArrayItem` (`self.PlayerStarts`))) "Undefined" "OverrideRootScale"))
    (`Controller.Possess` PlayerController _returnvalue_2)
    (else
      (bind _returnvalue_3 (`|SpawnActorFromClass` "/Game/VirtualRealityBP/Blueprints/MotionControllerPawn.MotionControllerPawn_C" (`self.GetTransform` (`|GetArrayItem` (`self.PlayerStarts`) 1)) "Undefined" "OverrideRootScale"))
      (`Controller.Possess` PlayerController _returnvalue_3))))

(event `self.K2_PostLogin`
  (params (NewPlayer :type "PlayerController Object Reference"))
  (`/Engine/EditorBlueprintResources/ActorMacros.Switch Has Authority`
    (:`Authority`
      (bind _outactors (`GameplayStatics.GetAllActorsOfClass` "/Script/Engine.PlayerStart"))
      (set `self.PlayerStarts` _outactors)
      (`self.RespawnPlayer` NewPlayer))))

(fn `UserConstructionScript`)