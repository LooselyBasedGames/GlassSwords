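; BP_BaseVRInstance is a game-instance-style Blueprint that enables the HMD on Init and handles basic multiplayer session hosting and joining.
; HostGameEvent creates a session using the EnableLAN setting, then opens the VRTest level on success.
; JoinSession searches with the same LAN setting and automatically joins the first result, with no selection step.
; Failures and empty searches only print a message.
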(event `self.ReceiveInit`
  (`HeadMountedDisplayFunctionLibrary.EnableHMD` true))

(event `HostGameEvent`
  (`CreateSessionCallbackProxy.CreateSession` (`GameplayStatics.GetPlayerController` 0) 0 (`self.EnableLAN`)
    (:`OnSuccess`
      (`GameplayStatics.OpenLevel` "VRTest"))
    (:`OnFailure`
      (`KismetSystemLibrary.PrintString` "Failed to create session"))))

(event `JoinSession`
  (bind _results (`FindSessionsCallbackProxy.FindSessions` (`GameplayStatics.GetPlayerController` 0) 10 (`self.EnableLAN`))
    (:`OnSuccess`
      (if (== (`KismetArrayLibrary.Array_Length` _results) 0)
        (`KismetSystemLibrary.PrintString` "No sessions found")
        (else
          (`JoinSessionCallbackProxy.JoinSession` (`GameplayStatics.GetPlayerController` 0) (`|GetArrayItem` _results)))))
    (:`OnFailure`
      (`KismetSystemLibrary.PrintString` "Rip"))))