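; VR sword actor that motion controllers pick up and drop, and that destroys itself when it overlaps another sword.
; Pickup records the holding hand, disables physics, shows the mesh at a per-hand offset, and snaps the root to the controller's attach component.
; Drop detaches the root and re-enables physics.
; Sword overlap plays haptics on the recorded hand and fires OnSwordDestroyed before destruction.
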(event `Event EnemySwordHit`
  (`KismetSystemLibrary.PrintString` "Overlapped other sword!")
  (`PlayerController.PlayHapticEffect` (`GameplayStatics.GetPlayerController` 0) "/Game/VirtualRealityBP/Blueprints/SwordDestroyedHaptics.SwordDestroyedHaptics" (`self.ParentHand`) 1.0 false)
  (`self.OnSwordDestroyed`)
  (`self.K2_DestroyActor`))

(event `self.ReceiveActorBeginOverlap`
  (params (OtherActor :type "Actor Object Reference"))
  (cast `/Game/Blueprints/BP_SwordPickup` OtherActor)
  (`self.Event EnemySwordHit`))

(event `/Game/VirtualRealityBP/Blueprints/PickupActorInterface.Pickup`
  (params (AttachTo :type "SceneComponent Object Reference"))
  (bind _staticmesh (`self.StaticMesh`))
  (bind _asbp_motion_controller (cast `/Game/VirtualRealityBP/Blueprints/BP_MotionController` (`ActorComponent.GetOwner` AttachTo)))
  (set `self.ParentHand` (`/Game/VirtualRealityBP/Blueprints/BP_MotionController.Hand` _asbp_motion_controller)) ; Store which hand is holding this sword
  (`SceneComponent.K2_AttachToComponent` _staticmesh (`self.DefaultSceneRoot`) "None" "KeepRelative" "KeepRelative" "KeepRelative" true)
  (`SceneComponent.K2_SetRelativeLocationAndRotation` :`self` (`self.StaticMesh`) :`NewLocation` (`self.GetLocationBasedOnHand` _asbp_motion_controller) :`bTeleport` true)
  (`PrimitiveComponent.SetSimulatePhysics` _staticmesh false)
  (`SceneComponent.K2_AttachToComponent` (`self.DefaultSceneRoot`) AttachTo "None" "SnapToTarget" "SnapToTarget" "KeepRelative" false)
  (`SceneComponent.SetVisibility` (`self.StaticMesh`) true false))

(event `/Game/VirtualRealityBP/Blueprints/PickupActorInterface.Drop`
  (`SceneComponent.K2_DetachFromComponent` (`self.DefaultSceneRoot`) "KeepRelative" "KeepRelative" "KeepRelative" true)
  (`PrimitiveComponent.SetSimulatePhysics` (`self.StaticMesh`) true))

(event `self.ReceiveBeginPlay`
  (set `self.MeshOffset` (`SceneComponent.RelativeLocation` (`self.StaticMesh`))))

(fn `GetLocationBasedOnHand`
  (params (MotionController :type "/Game/VirtualRealityBP/Blueprints/BP_MotionController Object Reference"))
  (returns (OffSet :type "Vector Structure"))
  (switch `EControllerHand` (`/Game/VirtualRealityBP/Blueprints/BP_MotionController.Hand` MotionController)
    (:`Left`
      (return (`self.LHOffset`)))
    (:`Right`
      (return (`self.RHOffset`)))
    (:`Pad`
      (return (0.0 0.0 0.0)))))

(fn `UserConstructionScript`)