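; VR player controller that asks the BaseVRMode game mode to respawn it on ClientPostLogin and handles hand grab input.
; GrabLeft and GrabRight press and release call Grab or Release events, which print debug text and forward to the matching motion controller on VRPawn.
; The cast that would set VRPawn from the controlled MotionControllerPawn is unconnected, so this graph never assigns that reference.
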(event `ClientPostLogin`
  (bind _asbase_vrmode (cast `/Game/Blueprints/GameModes/BaseVRMode` (`GameplayStatics.GetGameMode`)))
  (`/Game/Blueprints/GameModes/BaseVRMode.RespawnPlayer` _asbase_vrmode self))

(event `Grab`
  (params (Hand :type "/Game/VirtualRealityBP/Blueprints/BP_MotionController Object Reference"))
  (`KismetSystemLibrary.PrintString` "Should grab")
  (`/Game/VirtualRealityBP/Blueprints/BP_MotionController.Grab` Hand))

(event `Release`
  (params (Hand :type "/Game/VirtualRealityBP/Blueprints/BP_MotionController Object Reference"))
  (`KismetSystemLibrary.PrintString` "Should release")
  (`/Game/VirtualRealityBP/Blueprints/BP_MotionController.Release` Hand))

(event `InputAction|GrabLeft`
  (params (Key :type "Key Structure" :default "AnyKey"))
  (bind _leftcontroller (`/Game/VirtualRealityBP/Blueprints/MotionControllerPawn.LeftController` (`self.VRPawn`)))
  (:`Pressed`
    (`self.Grab` _leftcontroller))
  (:`Released`
    (`self.Release` _leftcontroller)))

(event `InputAction|GrabRight`
  (params (Key :type "Key Structure" :default "AnyKey"))
  (bind _rightcontroller (`/Game/VirtualRealityBP/Blueprints/MotionControllerPawn.RightController` (`self.VRPawn`)))
  (:`Pressed`
    (`self.Grab` _rightcontroller))
  (:`Released`
    (`self.Release` _rightcontroller)))

(event `self.ReceiveBeginPlay`
  (`KismetSystemLibrary.PrintString` "Begin play called"))

(fn `UserConstructionScript`)