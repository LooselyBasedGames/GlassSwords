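; BP_SwordPickup is a VR sword that can be picked up and dropped, and is destroyed when it clashes with another equipped sword.
; Pickup marks it equipped and routes through server and multicast events to attach the mesh with physics off; Drop detaches and restores physics.
; Mesh overlaps register hits only after a short spawn delay when both swords are equipped, triggering haptics, destruction and OnSwordDestroyed.
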(event `self.ReceiveBeginPlay`
  (`KismetSystemLibrary.Delay` 0.2)
  (set `self.IsActive` true))

(event `Event EnemySwordHit`
  (set `self.IsPendingKill` true)
  (`KismetSystemLibrary.PrintString` "Overlapped other sword!")
  (`PlayerController.PlayHapticEffect` (`GameplayStatics.GetPlayerController` 0) "/Game/VirtualRealityBP/Blueprints/SwordDestroyedHaptics.SwordDestroyedHaptics" (`self.ParentHand`) 1.0 false)
  (`self.K2_DestroyActor`)
  (`self.OnSwordDestroyed`))

(event `self.ReceiveActorBeginOverlap`
  (params (OtherActor :type "Actor Object Reference")))

(event `ServerPickup`
  (params (AttachTo :type "SceneComponent Object Reference"))
  (`self.HandlePickup` AttachTo)
  (`self.MulticastPickup` AttachTo))

(event `HandlePickup`
  (params (AttachTo :type "SceneComponent Object Reference"))
  (`SceneComponent.K2_AttachToComponent` (`self.StaticMesh`) AttachTo "None" "KeepRelative" "KeepRelative" "KeepWorld" true)
  (`SceneComponent.K2_SetRelativeLocationAndRotation` (`self.StaticMesh`) (- (`SceneComponent.K2_GetComponentLocation` AttachTo) (200.0 40.0 300.0)) (struct :`Pitch` -45.0) false true)
  (`PrimitiveComponent.SetSimulatePhysics` (`self.StaticMesh`) false)
  (`SceneComponent.SetVisibility` (`self.StaticMesh`) true false))

(event `/Game/VirtualRealityBP/Blueprints/PickupActorInterface.Pickup`
  (params (AttachTo :type "SceneComponent Object Reference"))
  (set `self.IsEquipped` true)
  (`self.ServerPickup` AttachTo))

(event `MulticastPickup`
  (params (`Attach To` :type "SceneComponent Object Reference"))
  (`self.HandlePickup` `Attach To`))

(event `/Game/VirtualRealityBP/Blueprints/PickupActorInterface.Drop`
  (`SceneComponent.K2_DetachFromComponent` (`self.StaticMesh`) "KeepRelative" "KeepRelative" "KeepRelative" true)
  (`PrimitiveComponent.SetSimulatePhysics` (`self.StaticMesh`) true))

(event `UpdateSwordLocationRotation`
  (params (Location :type "Vector Structure") (Rotation :type "Rotator Structure"))
  (`SceneComponent.K2_SetWorldLocationAndRotation` (`self.StaticMesh`) Location Rotation true false))

(event `self.StaticMesh.OnComponentBeginOverlap`
  (params (OverlappedComponent :type "PrimitiveComponent Object Reference") (OtherActor :type "Actor Object Reference") (OtherComp :type "PrimitiveComponent Object Reference") (OtherBodyIndex :type Integer) (bFromSweep :type Boolean) (SweepResult :type "HitResult Structure (by ref)"))
  (bind _asbp_sword_pickup (cast `/Game/Blueprints/Environment/BP_SwordPickup` OtherActor))
  (if (`self.ShouldRegisterHit` _asbp_sword_pickup)
    (`self.Event EnemySwordHit`)))

(fn `GetLocationBasedOnHand`
  (params (MotionController :type "/Game/VirtualRealityBP/Blueprints/BP_MotionController Object Reference"))
  (returns (OffSet :type "Vector Structure"))
  (switch `EControllerHand` (`/Game/VirtualRealityBP/Blueprints/BP_MotionController.Hand` MotionController)
    (:`Left`
      (return (`self.LHOffset`)))
    (:`Right`
      (return (`self.RHOffset`)))
    (:`Pad`
      (return (0.0 0.0 0.0)))))

(fn `ShouldRegisterHit`
  (params (HitSword :type "/Game/Blueprints/Environment/BP_SwordPickup Object Reference"))
  (returns (Value :type Boolean))
  (if (not (`self.IsActive`))
    (return false)
    (elif (or (`self.IsPendingKill`) (`/Game/Blueprints/Environment/BP_SwordPickup.IsPendingKill` HitSword))
      (return false)
      (else
        (return (and (`/Game/Blueprints/Environment/BP_SwordPickup.IsEquipped` HitSword) (`self.IsEquipped`)))))))

(fn `UserConstructionScript`)