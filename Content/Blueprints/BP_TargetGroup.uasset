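; BP_TargetGroup is an actor holding three targets that disappear when a sword pickup touches them.
; Each target component has its own begin-overlap event that casts the other actor to BP_SwordPickup and ignores anything else.
; A hit deactivates and hides that single target without propagating to children; collision is not changed, and nothing is counted or reset.
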(event `self.Target1.OnComponentBeginOverlap`
  (params (OverlappedComponent :type "PrimitiveComponent Object Reference") (OtherActor :type "Actor Object Reference") (OtherComp :type "PrimitiveComponent Object Reference") (OtherBodyIndex :type Integer) (bFromSweep :type Boolean) (SweepResult :type "HitResult Structure (by ref)"))
  (cast `/Game/Blueprints/BP_SwordPickup` OtherActor)
  (`ActorComponent.SetActive` (`self.Target1`) false false)
  (`SceneComponent.SetVisibility` (`self.Target1`) false false))

(event `self.Target2.OnComponentBeginOverlap`
  (params (OverlappedComponent :type "PrimitiveComponent Object Reference") (OtherActor :type "Actor Object Reference") (OtherComp :type "PrimitiveComponent Object Reference") (OtherBodyIndex :type Integer) (bFromSweep :type Boolean) (SweepResult :type "HitResult Structure (by ref)"))
  (cast `/Game/Blueprints/BP_SwordPickup` OtherActor)
  (`ActorComponent.SetActive` (`self.Target2`) false false)
  (`SceneComponent.SetVisibility` (`self.Target2`) false false))

(event `self.Target3.OnComponentBeginOverlap`
  (params (OverlappedComponent :type "PrimitiveComponent Object Reference") (OtherActor :type "Actor Object Reference") (OtherComp :type "PrimitiveComponent Object Reference") (OtherBodyIndex :type Integer) (bFromSweep :type Boolean) (SweepResult :type "HitResult Structure (by ref)"))
  (cast `/Game/Blueprints/BP_SwordPickup` OtherActor)
  (`ActorComponent.SetActive` (`self.Target3`) false false)
  (`SceneComponent.SetVisibility` (`self.Target3`) false false))

(fn `UserConstructionScript`)