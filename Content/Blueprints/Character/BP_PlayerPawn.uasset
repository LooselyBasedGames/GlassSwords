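; BP_PlayerPawn is a networked VR player pawn that syncs head and hand motion and handles swords.
; Each tick, the local player relays camera and motion-controller transforms through server-to-client events, applied only on non-owning machines.
; Sword spawning and right-hand grabbing use the same relay, with destroyed swords replaced at SwordSpawnLocation.
; The local head is hidden, remote heads are tinted red, and right-hand sword overlaps play haptics.
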(event `Clients_UpdateLocationRotation`
  (params (Component :type "SceneComponent Object Reference") (RelativeLoc :type "Vector Structure") (`Relative Rot` :type "Rotator Structure"))
  (if (not (`self.IsLocallyControlled`))
    (`SceneComponent.K2_SetRelativeLocationAndRotation` Component RelativeLoc `Relative Rot` false false)))

(event `Server_UpdateLocationRotation`
  (params (Component :type "SceneComponent Object Reference") (RelativeLoc :type "Vector Structure") (RelativeRot :type "Rotator Structure"))
  (`self.Clients_UpdateLocationRotation` Component RelativeLoc RelativeRot))

(event `UpdateHeadOnClients`
  (params (Loc :type "Vector Structure") (Rot :type "Rotator Structure"))
  (`SceneComponent.K2_SetWorldLocationAndRotation` (`self.Head`) Loc (`KismetMathLibrary.MakeRotator` Rot_Roll Rot_Pitch (- Rot_Yaw 90.0)) false false))

(event `UpdateHeadLocationAndRotation`
  (params (WorldRot :type "Rotator Structure") (WorldLoc :type "Vector Structure"))
  (`self.UpdateHeadOnClients` WorldLoc WorldRot))

(event `self.ReceiveTick`
  (params (DeltaSeconds :type "Float (single-precision)"))
  (bind _camera (`self.Camera`))
  (bind _rmc (`self.RMC`))
  (bind _lmc (`self.LMC`))
  (bind (_relativerotation_roll _relativerotation_pitch _relativerotation_yaw) (`KismetMathLibrary.BreakRotator` (`SceneComponent.RelativeRotation` _camera)))
  (if (`self.IsLocallyControlled`)
    (`self.Server_UpdateLocationRotation` _camera (`SceneComponent.RelativeLocation` _camera) (`KismetMathLibrary.MakeRotator` _relativerotation_roll _relativerotation_pitch (- _relativerotation_yaw 90.0)))
    (`self.Server_UpdateLocationRotation` (`self.RightSphere`) (`SceneComponent.RelativeLocation` _rmc) (`SceneComponent.RelativeRotation` _rmc))
    (`self.Server_UpdateLocationRotation` (`self.LeftSphere`) (`SceneComponent.RelativeLocation` _lmc) (`SceneComponent.RelativeRotation` _lmc))))

(event `self.ReceiveBeginPlay`
  (if (`self.IsLocallyControlled`)
    (`SceneComponent.SetVisibility` (`self.Head`) false false)
    (`self.Server_EquipNewSword`)
    (else
      (bind _returnvalue (`PrimitiveComponent.CreateDynamicMaterialInstance` (`self.Head`) 0 null))
      (`MaterialInstanceDynamic.SetVectorParameterValue` _returnvalue "Color" (struct :`R` 0.77 :`A` 1.0)))))

(event `ClientUpdateSwordLocationRotation`
  (params (Sword :type "/Game/Blueprints/BP_SwordPickup Object Reference"))
  (`self.K2_AttachToComponent` Sword (`self.SwordSpawnLocation`) "None" "SnapToTarget" "SnapToTarget" "KeepRelative" false)
  (`SceneComponent.SetVisibility` (`/Game/Blueprints/BP_SwordPickup.StaticMesh` Sword) true false))

(event `ServerPickup`
  (params (AttachTo :type "SceneComponent Object Reference"))
  (`self.MultiPickup` AttachTo))

(event `MultiPickup`
  (params (AttachTo :type "SceneComponent Object Reference"))
  (`KismetSystemLibrary.PrintString` "Grip")
  (bind _outactors (`KismetSystemLibrary.SphereOverlapActors` (`SceneComponent.K2_GetComponentLocation` AttachTo) 30.0 (`self.Types`) "/Game/Blueprints/BP_SwordPickup.BP_SwordPickup_C"))
  (bind _output (`|GetArrayItem` _outactors))
  (`KismetSystemLibrary.PrintString` (`KismetSystemLibrary.GetDisplayName` _output))
  (message `/Game/VirtualRealityBP/Blueprints/PickupActorInterface.Pickup` _output AttachTo))

(event `InputAction|GrabRight`
  (params (Key :type "Key Structure" :default "AnyKey"))
  (:`Pressed`
    (if (`self.IsLocallyControlled`)
      (`self.ServerPickup` (`self.RightSphere`)))))

(event `Server_EquipNewSword`
  (`self.Multi_EquipNewSword`))

(event `Multi_EquipNewSword`
  (bind _returnvalue (`|SpawnActorFromClass` "/Game/Blueprints/BP_SwordPickup.BP_SwordPickup_C" (`SceneComponent.K2_GetComponentToWorld` (`self.SwordSpawnLocation`)) "Undefined" "OverrideRootScale"))
  (`self.EquipSword` _returnvalue))

(event `EquipSword`
  (params (Sword :type "/Game/Blueprints/BP_SwordPickup Object Reference"))
  (add `/Game/Blueprints/BP_SwordPickup.OnSwordDestroyed` Sword (delegate `HandleSwordDestroyed`))
  (`self.K2_AttachToComponent` Sword (`self.SwordSpawnLocation`) "None" "SnapToTarget" "SnapToTarget" "KeepRelative" false))

(event `HandleSwordDestroyed`
  (`self.Server_EquipNewSword`))

(event `self.RMC.OnComponentBeginOverlap`
  (params (OverlappedComponent :type "PrimitiveComponent Object Reference") (OtherActor :type "Actor Object Reference") (OtherComp :type "PrimitiveComponent Object Reference") (OtherBodyIndex :type Integer) (bFromSweep :type Boolean) (SweepResult :type "HitResult Structure (by ref)")))

(event `self.RightSphere.OnComponentBeginOverlap`
  (params (OverlappedComponent :type "PrimitiveComponent Object Reference") (OtherActor :type "Actor Object Reference") (OtherComp :type "PrimitiveComponent Object Reference") (OtherBodyIndex :type Integer) (bFromSweep :type Boolean) (SweepResult :type "HitResult Structure (by ref)"))
  (cast `/Game/Blueprints/BP_SwordPickup` OtherActor)
  (`PlayerController.PlayHapticEffect` (`GameplayStatics.GetPlayerController` 0) "/Game/VirtualRealityBP/Blueprints/ItemHoverHaptics.ItemHoverHaptics" "Right" 1.0 false))

(fn `UserConstructionScript`)